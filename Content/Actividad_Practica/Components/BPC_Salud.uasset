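; BPC_Salud is a health component that holds an actor's current and total health.
; Daño subtracts damage and Cura adds healing, each clamping VidaActual between zero and VidaTotal.
; Each function then broadcasts its dispatcher, RecibirDaño or RecibirCura, with current and total health so bound listeners can react.
; It has no death handling and no active BeginPlay or Tick logic.
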(fn `Cura`
  (params (Cura :type "Float (double-precision)"))
  (set `self.VidaActual` (`KismetMathLibrary.FClamp` (+ (`self.VidaActual`) Cura) 0.0 (`self.VidaTotal`)))
  (`self.Recibir Cura` (`self.VidaActual`) (`self.VidaTotal`)))

(fn `Daño`
  (params (`Daño` :type "Float (double-precision)"))
  (set `self.VidaActual` (`KismetMathLibrary.FClamp` (- (`self.VidaActual`) `Daño`) 0.0 (`self.VidaTotal`)))
  (`self.RecibirDaño` (`self.VidaActual`) (`self.VidaTotal`)))